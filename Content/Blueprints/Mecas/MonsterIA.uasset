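; MonsterIA is a monster AI Blueprint that rises, wanders and chases pawns it sees.
; On BeginPlay it plays a zombie stand-up animation, starts wandering after a delay, then switches the mesh to the MonsterAnim class.
; Wandering chains AI moves to random reachable nearby points, repeating only on success.
; PawnSensing sightings redirect movement to the seen pawn, while a retriggerable delay resumes wandering shortly after sightings stop.
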(event OnSeePawn(PawnSensing)
  (params (Pawn :type Pawn%20Object%20Reference))
  (Utilities|FlowControl|Sequence
    (:then_0
      (AI|AIMoveTo self "0, 0, 0" Pawn 5.0 false))
    (:then_1
      (Utilities|FlowControl|RetriggerableDelay 1.0)
      (CallFunction|MovetoRandomLocation))))

(event Custom|Up
  (bind _mesh (Variables|Character|GetMesh))
  (Components|Animation|PlayAnimation _mesh "/Game/Characters/Monster/Animation/SpaceElemental_Zombie_Stand_Up.SpaceElemental_Zombie_Stand_Up" false)
  (Utilities|FlowControl|Delay 3.0)
  (CallFunction|MovetoRandomLocation)
  (Class|SkeletalMeshComponent|SetAnimClass _mesh "/Game/Characters/Monster/MonsterAnim.MonsterAnim_C"))

(event Custom|MoveToRandomLocation
  (AI|AIMoveTo self (.RandomLocation (AI|Navigation|GetRandomReachablePointinRadius (Transformation|GetActorLocation) 1.5e+03 0 0)) 0 5.0 false
    (:OnSuccess
      (CallFunction|MovetoRandomLocation))))

(event EventBeginPlay
  (CallFunction|Up))

(event Collision|EventActorBeginOverlap
  (params (OtherActor :type Actor%20Object%20Reference)))

(event EventTick
  (params (DeltaSeconds :type Float%20%28single-precision%29)))

(fn ConstructionScript)