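; Blink_Ligth is a point light that flickers constantly and suffers periodic timed blackouts.
; Tick runs a random short Delay before toggling the light's visibility, producing an irregular blink.
; A looping timer from BeginPlay calls Blackout, which, if LumiereActive is true, zeroes intensity and schedules LigthOn to restore it seconds later.
; Both timed events call GetAllActorsOfClass without visibly using the result, and LigthOn assigns LumiereActive to itself.
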(event Custom|Blackout
  (if (Variables|Default|GetLumiere%20active%20?)
    (Actor|GetAllActorsOfClass "Blink_Ligth_C")
    (Rendering|Components|Light|SetIntensity (Variables|Default|GetPointLight) 0.0)
    (Utilities|Time|SetTimerbyFunctionName 0 "LigthOn" 5.0)))

(event Custom|LigthOn
  (Actor|GetAllActorsOfClass "Blink_Ligth_C")
  (Rendering|Components|Light|SetIntensity (Variables|Default|GetPointLight) 3e+02)
  (Variables|Default|SetLumiere%20active%20? (Variables|Default|GetLumiere%20active%20?)))

(event EventBeginPlay
  (Utilities|Time|SetTimerbyFunctionName 0 "Blackout " 1.2e+02 true))

(event EventTick
  (params (DeltaSeconds :type Float%20%28single-precision%29))
  (Utilities|FlowControl|Delay (Math|Random|RandomFloatinRange 0.1 1.0))
  (Rendering|ToggleVisibility (Variables|Default|GetPointLight) false))

(fn ConstructionScript)